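; Trash spawner actor that periodically drops trash actors at random points inside its SpawnArea box.
; On BeginPlay it caches the game instance and starts a looping timer, which Deactivate clears.
; Each tick of the timer spawns TrashClass only while the game instance's shared TrashArray is below MaxSpawnedTrash, then registers it there.
; A downward visibility trace snaps each new piece onto the surface below.
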(event EventBeginPlay
  (bind _asescape_in_space_game_instance (Utilities|Casting|CastToEscapeInSpaceGameInstance (Game|GetGameInstance)))
  (Variables|Default|SetAs%20Escape%20In%20Space%20Game%20Instance _asescape_in_space_game_instance)
  (Variables|Default|SetTrash%20Array (Variables|/Game/Blueprints/EscapeInSpaceGameInstance.EscapeInSpaceGameInstance_C|GetTrashArray _asescape_in_space_game_instance))
  (CallFunction|Activate))

(event Collision|EventActorBeginOverlap
  (params (OtherActor :type Actor%20Object%20Reference)))

(event EventTick
  (params (DeltaSeconds :type Float%20%28single-precision%29)))

(fn ConstructionScript)

(fn Activate
  (Variables|Default|SetIsActive true)
  (bind _returnvalue (Utilities|Time|SetTimerbyFunctionName 0 "TrySpawnTrash" 4.0 true))
  (Variables|Default|SetTrashSpawnTimer _returnvalue))

(fn Deactivate
  (Variables|Default|SetIsActive false)
  (Utilities|Time|ClearandInvalidateTimerbyHandle (Variables|Default|GetTrashSpawnTimer)))

(fn TrySpawnTrash
  (bind _spawnarea (Variables|Default|GetSpawnArea))
  (if (< (Utilities|Array|Length (Variables|/Game/Blueprints/EscapeInSpaceGameInstance.EscapeInSpaceGameInstance_C|GetTrashArray (Variables|Default|GetAs%20Escape%20In%20Space%20Game%20Instance))) (Variables|Default|GetMaxSpawnedTrash))
    (bind _returnvalue (Game|SpawnActorfromClass (Variables|Default|GetTrashClass) (Math|Transform|MakeTransform (Math|Random|RandomPointinBoundingBox (Transformation|GetWorldLocation _spawnarea) (Components|Box|GetScaledBoxExtent _spawnarea)) "0, 0, 0" "1.000000,1.000000,1.000000") "Undefined" "MultiplyWithRoot" 0 0))
    (Utilities|IsValid _returnvalue
      (:Is%20Valid
        (bind _output_get (Variables|Default|SetLastSpawnedTrash _returnvalue))
        (Utilities|Array|Add (Variables|/Game/Blueprints/EscapeInSpaceGameInstance.EscapeInSpaceGameInstance_C|GetTrashArray (Variables|Default|GetAs%20Escape%20In%20Space%20Game%20Instance)) _output_get)
        (bind (_outhit _returnvalue_2) (Collision|LineTraceByChannel (Transformation|GetActorLocation _returnvalue) (- (Transformation|GetActorLocation _returnvalue) "0.000000,0.000000,1000.000000") "TraceTypeQuery1" false 0 "None"))
        (if _returnvalue_2
          (Transformation|SetActorLocation (Variables|Default|GetLastSpawnedTrash) (.Location (Collision|BreakHitResult _outhit)) false false))))))